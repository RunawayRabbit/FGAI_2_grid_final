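; Player controller that handles mouse input for selecting units and ordering them to move, RTS-style.
; Left mouse press and release are forwarded to the FGHUD as select events.
; Right click traces under the cursor on the Visibility channel and, on a hit, sends every unit in SelectedUnits a MoveTo to that same location.
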(event Input|MouseEvents|LeftMouseButton
  (params (Key :type Key%20Structure :default "None"))
  (bind _returnvalue (HUD|GetHUD))
  (:Pressed
    (bind _asfghud (Utilities|Casting|CastToFGHUD _returnvalue))
    (Class|FGHUD|OnSelectPress _asfghud))
  (:Released
    (bind _asfghud_2 (Utilities|Casting|CastToFGHUD _returnvalue))
    (Class|FGHUD|OnSelectRelease _asfghud_2)))

(event Input|MouseEvents|RightMouseButton
  (params (Key :type Key%20Structure :default "None"))
  (bind (_hitresult _returnvalue) (Game|Player|GetHitResultUnderCursorbyChannel "TraceTypeQuery1" true))
  (:Pressed
    (if _returnvalue
      (Variables|Default|SetLocation (.Location (Collision|BreakHitResult _hitresult)))
      (for _array_element (Variables|Default|GetSelectedUnits)
        (Class|FGDude|Moveto _array_element (Variables|Default|GetLocation))))))

(fn ConstructionScript)