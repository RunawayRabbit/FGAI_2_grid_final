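; BP_Player is a player Blueprint for picking and debugging start and end positions on a tile grid.
; Each tick, while the mouse is over the grid, it draws debug spheres at the cursor, the start in green and the end in red.
; SetStart and SetEnd store a position and call DrawNeighbours, which converts it to tile coordinates through the current grid actor and prints the neighbour count.
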(event EventTick
  (params (DeltaSeconds :type Float%20%28single-precision%29))
  (bind (_outworldmouselocation _returnvalue) (Class|FGPlayer|GetMouseLocationonGrid))
  (if _returnvalue
    (Rendering|Debug|DrawDebugSphere _outworldmouselocation 1e+02 12 "(R=1.000000,G=1.000000,B=1.000000,A=1.000000)" 0.0)
    (Rendering|Debug|DrawDebugSphere (Variables|Default|GetStartPos) 1e+02 12 "(R=0.000000,G=0.723958,B=0.086970,A=1.000000)" 0.0)
    (Rendering|Debug|DrawDebugSphere (Variables|Default|GetEndPos) 1e+02 12 "(R=0.713542,G=0.006953,B=0.000000,A=1.000000)" 0.0)))

(event EventSetEnd
  (params (Position :type Vector :default "0, 0, 0"))
  (bind _output_get (Variables|Default|SetEndPos Position))
  (CallFunction|DrawNeighbours _output_get))

(event EventSetStart
  (params (Position :type Vector :default "0, 0, 0"))
  (bind _output_get (Variables|Default|SetStartPos Position))
  (CallFunction|DrawNeighbours _output_get))

(fn ConstructionScript)

(fn DrawNeighbours
  (params (Location :type Vector))
  (bind _currentgridactor (Variables|Default|GetCurrentGridActor))
  (bind (_tilex _tiley _returnvalue) (Class|FGGridActor|GetXYfromWorldLocation _currentgridactor Location))
  (if _returnvalue
    (Development|PrintString (Utilities|String|ToString(Integer) (Utilities|Array|Length (Class|FGGridActor|GetNeighbours _currentgridactor (Utilities|Struct|MakeVector2Int _tilex _tiley)))))))